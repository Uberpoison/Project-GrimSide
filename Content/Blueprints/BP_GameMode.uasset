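; Game mode that resets the level's characters when the player dies.
; It caches the player character on BeginPlay, checks for death every Tick, then delays for the death animation length plus a short pause.
; After the delay it calls Respawn on every base character, player and enemies alike, and clears the rewind arrays on all enemy controllers.
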(event `self.ReceiveBeginPlay`
  (bind _returnvalue (`GameplayStatics.GetPlayerPawn` 0))
  (`/Engine/EditorBlueprintResources/StandardMacros.IsValid` _returnvalue
    (:`Is Valid`
      (bind _asbp_player_character (cast `/Game/Blueprints/BP_PlayerCharacter` _returnvalue))
      (set `self.Player` _asbp_player_character))))

(event `self.ReceiveTick`
  (params (DeltaSeconds :type "Float (single-precision)"))
  (if (`self.IsPlayerDead`)
    (`KismetSystemLibrary.Delay` (+ (`self.GetLengthOfCurrentDeathAnim`) 3.5))
    ;[1 1 1] Respawn Player and Enemies
    (bind _outactors (`GameplayStatics.GetAllActorsOfClass` "/Game/Blueprints/BP_BaseCharacter.BP_BaseCharacter_C"))
    (for _array_element _outactors
      (`/Game/Blueprints/BP_BaseCharacter.Respawn` _array_element))
    ;[1 1 1] Clear Rewind Data of the Enemies
    (bind _outactors_2 (`GameplayStatics.GetAllActorsOfClass` "/Game/Blueprints/AI/BP_BaseEnemyController.BP_BaseEnemyController_C"))
    (for _array_element_2 _outactors_2
      (`/Game/Blueprints/AI/BP_BaseEnemyController.ClearRewindArrays` _array_element_2))))

(fn `UserConstructionScript`)