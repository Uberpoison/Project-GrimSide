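; Health component that tracks current and maximum health for its owner and resets to full on BeginPlay.
; DoDamage clamps health between zero and max, so negative amounts heal, and returns whether the owner is dead.
; It fires OnDeath only when a hit lowers health to zero, and OnTakingDamage on every call with amount, impact point and normal.
; Helper functions expose health percentage and death state.
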(event `self.ReceiveBeginPlay`
  (`self.ResetHealth`))

(event `ResetHealth`
  (set `self.CurrentHealth` (`self.MaxHealth`)))

(fn `Do Damage`
  (params (Amount :type "Float (double-precision)") (ImpactPoint :type "Vector Structure") (ImpactNormal :type "Vector Structure"))
  (returns (IsDead :type Boolean))
  (bind _isdead (`self.IsDead`))
  (bind _currenthealth (`self.CurrentHealth`))
  (set `self.OriginalHealth` _currenthealth)
  (bind _output_get (set `self.CurrentHealth` (`KismetMathLibrary.FClamp` (- _currenthealth Amount) 0.0 (`self.MaxHealth`))))
  ;[1 1 1] Did this DoDamage cause the health to change and drop to 0??
  (if (and _isdead (> (`self.OriginalHealth`) _output_get))
    (`self.OnDeath`))
  (`self.OnTakingDamage` Amount ImpactPoint ImpactNormal)
  (return _isdead))

(fn `GetHealthPercentage`
  (returns (HealthPercentage :type "Float (double-precision)"))
  (return (/ (`self.CurrentHealth`) (`self.MaxHealth`))))

(fn `IsDead`
  (returns (IsDead :type Boolean))
  (return (== (`self.GetHealthPercentage`) 0.0)))