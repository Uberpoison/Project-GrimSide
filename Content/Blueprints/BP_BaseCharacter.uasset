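; Base character Blueprint providing lock-on targeting, health bar display and respawn behavior.
; Health bar and lock-on widget components toggle visibility, with the health bar bound to this character and Lockon flip-flopping the targeted state.
; DistanceToPlayer line-traces to the player pawn, storing hit distance and unconditionally marking the character targetable.
; Respawn restores the transform saved at BeginPlay or via SetSpawnPoint, resets BPCHealth and stops playing montages.
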(event `self.ReceiveBeginPlay`
  (set `self.SpawnPoint` (`self.GetTransform`)))

(event `self.ReceiveTick`
  (params (DeltaSeconds :type "Float (single-precision)")))

(event `/Game/Blueprints/BPI_LockOnSystem.LockOn`
  (`/Engine/EditorBlueprintResources/StandardMacros.FlipFlop`
    (:`A`
      (`self.ShowLockOn` true)
      (set `self.IsTargeted` true))
    (:`B`
      (`self.ShowLockOn` false)
      (set `self.IsTargeted` false))))

(fn `DistanceToPlayer`
  (bind _outhit (`KismetSystemLibrary.LineTraceSingleForObjects` (`self.K2_GetActorLocation`) (`self.K2_GetActorLocation` (`GameplayStatics.GetPlayerPawn` 0)) (`|MakeArray` "ObjectTypeQuery3" :!type "EObjectTypeQuery Enum") false (`|MakeArray` self :!type "Actor Object Reference") "None" true (struct :`R` 1.0 :`A` 1.0) (struct :`G` 1.0 :`A` 1.0) 0.1))
  (set `self.PlayerToEnemyDistance` (`.Distance` (`GameplayStatics.BreakHitResult` _outhit)))
  (set `self.CanBeTargeted` true))

(fn `Respawn`
  (bind _returnvalue (`SkeletalMeshComponent.GetAnimInstance` (`self.Mesh`)))
  (`self.K2_SetActorTransform` (`self.SpawnPoint`))
  (`/Game/Blueprints/BPC_Health.ResetHealth` (`self.BPC_Health`))
  (if (`AnimInstance.IsAnyMontagePlaying` _returnvalue)
    (`AnimInstance.StopSlotAnimation` _returnvalue 0.0 "None")))

(fn `SetSpawnPoint`
  (params (`New SpawnPoint` :type "Transform Structure"))
  (set `self.SpawnPoint` `New SpawnPoint`))

(fn `ShowHealthBar`
  (params (Enable :type Boolean))
  (bind _healthbar (`self.HealthBar`))
  (bind _asbp_enemy_health_bar (cast `/Game/Blueprints/AI/BP_EnemyHealthBar` (`WidgetComponent.GetUserWidgetObject` _healthbar)))
  (set `/Game/Blueprints/AI/BP_EnemyHealthBar.Enemy` self _asbp_enemy_health_bar)
  (`SceneComponent.SetVisibility` _healthbar Enable false))

(fn `ShowLockOn`
  (params (Enable :type Boolean))
  (bind _lockonsymbol (`self.LockOnSymbol`))
  (cast `/Game/Blueprints/AI/BP_LockOn` (`WidgetComponent.GetUserWidgetObject` _lockonsymbol))
  (`SceneComponent.SetVisibility` _lockonsymbol Enable false))

(fn `UserConstructionScript`)