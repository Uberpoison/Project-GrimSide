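; Animation notify state that deals melee weapon damage during the attack window of an animation.
; Each tick it sphere-traces on the Camera channel between the owning BP_BaseCharacter weapon's BladeBottom and BladeTop.
; A hit character with a BPC_Health component and CanBeHit takes the weapon's damage, unless both sides are tagged Enemy.
; Damaged actors join HitActors, which the trace ignores until NotifyEnd clears it, preventing repeat hits.
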(fn `Received_NotifyEnd`
  (params (MeshComp :type "SkeletalMeshComponent Object Reference") (Animation :type "AnimSequenceBase Object Reference"))
  (returns (ReturnValue :type Boolean))
  (`KismetArrayLibrary.Array_Clear` (`self.HitActors`))
  (return false))

(fn `Received_NotifyTick`
  (params (MeshComp :type "SkeletalMeshComponent Object Reference") (Animation :type "AnimSequenceBase Object Reference") (FrameDeltaTime :type "Float (double-precision)"))
  (returns (ReturnValue :type Boolean))
  (locals (OwnerActor :type "/Game/Blueprints/BP_BaseCharacter Object Reference") (HitActor :type "/Game/Blueprints/BP_BaseCharacter Object Reference"))
  ;[1 1 1] Sphere trace along the length of the blade and check what it hits and ignore actor if already hit in this notify
  (bind _asbp_base_character (cast `/Game/Blueprints/BP_BaseCharacter` (`AnimInstance.TryGetPawnOwner` (`SkeletalMeshComponent.GetAnimInstance` MeshComp))))
  (set `local.OwnerActor` _asbp_base_character)
  (bind _currentweapon (`/Game/Blueprints/BP_BaseCharacter.CurrentWeapon` _asbp_base_character))
  (bind (_outhit _returnvalue) (`KismetSystemLibrary.SphereTraceSingle` MeshComp (`SceneComponent.GetSocketLocation` (`/Game/Blueprints/BP_BaseWeapon.BladeBottom` _currentweapon) "None") (`SceneComponent.GetSocketLocation` (`/Game/Blueprints/BP_BaseWeapon.BladeTop` _currentweapon) "None") 15.0 "TraceTypeQuery2" false (`self.HitActors`)))
  (if _returnvalue
    ;[1 1 1] Check if we hit an actor
    (`/Engine/EditorBlueprintResources/StandardMacros.IsValid` (`.HitActor` (`GameplayStatics.BreakHitResult` _outhit))
      (:`Is Valid`
        (bind _returnvalue_2 (`Actor.GetComponentByClass` (`.HitActor` (`GameplayStatics.BreakHitResult` _outhit)) "/Game/Blueprints/BPC_Health.BPC_Health_C"))
        ;[1 1 1] Check if that actor has a Health component
        (`/Engine/EditorBlueprintResources/StandardMacros.IsValid` _returnvalue_2
          (:`Is Valid`
            (bind _asbp_base_character_2 (cast `/Game/Blueprints/BP_BaseCharacter` (`.HitActor` (`GameplayStatics.BreakHitResult` _outhit))))
            (set `local.HitActor` _asbp_base_character_2)
            (if (`/Game/Blueprints/BP_BaseCharacter.CanBeHit` _asbp_base_character_2)
              (if (not (and (`Actor.ActorHasTag` (`local.OwnerActor`) "Enemy") (`Actor.ActorHasTag` (`local.HitActor`) "Enemy")))
                (bind _isdead (`/Game/Blueprints/BPC_Health.Do Damage` _returnvalue_2 (`/Game/Blueprints/BP_BaseWeapon.Damage` _currentweapon) (`.ImpactPoint` (`GameplayStatics.BreakHitResult` _outhit)) (`.ImpactNormal` (`GameplayStatics.BreakHitResult` _outhit))))
                ;[1 1 1] Add actor to the array of hit actors
                (`KismetArrayLibrary.Array_Add` (`self.HitActors`) (`.HitActor` (`GameplayStatics.BreakHitResult` _outhit)))
                (return _isdead)))))))))