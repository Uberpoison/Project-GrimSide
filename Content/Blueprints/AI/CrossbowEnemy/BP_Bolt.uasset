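; BP_Bolt is a crossbow enemy projectile that damages the player on contact.
; Each Tick it sphere-traces between its Top and Bottom components on the Camera channel instead of using overlap events.
; A hit on a non-Enemy BP_PlayerCharacter with CanBeHit applies Damage through BPC_Health, then destroys the bolt.
; A trace hit without a valid actor destroys it after a delay.
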(event `self.ReceiveActorBeginOverlap`
  (params (OtherActor :type "Actor Object Reference")))

(event `self.ReceiveTick`
  (params (DeltaSeconds :type "Float (single-precision)"))
  (bind (_outhit _returnvalue) (`KismetSystemLibrary.SphereTraceSingle` (`SceneComponent.GetSocketLocation` (`self.Top`) "None") (`SceneComponent.GetSocketLocation` (`self.Bottom`) "None") 5.0 "TraceTypeQuery2"))
  (if _returnvalue
    (`/Engine/EditorBlueprintResources/StandardMacros.IsValid` (`.HitActor` (`GameplayStatics.BreakHitResult` _outhit))
      (:`Is Valid`
        (bind _returnvalue_2 (`self.GetComponentByClass` (`.HitActor` (`GameplayStatics.BreakHitResult` _outhit)) "/Game/Blueprints/BPC_Health.BPC_Health_C"))
        (`/Engine/EditorBlueprintResources/StandardMacros.IsValid` _returnvalue_2
          (:`Is Valid`
            (if (not (`self.ActorHasTag` (`.HitActor` (`GameplayStatics.BreakHitResult` _outhit)) "Enemy"))
              (bind _asbp_player_character (cast `/Game/Blueprints/BP_PlayerCharacter` (`.HitActor` (`GameplayStatics.BreakHitResult` _outhit))))
              (if (`/Game/Blueprints/BP_BaseCharacter.CanBeHit` _asbp_player_character)
                (`/Game/Blueprints/BPC_Health.Do Damage` _returnvalue_2 (`self.Damage`) (`.ImpactPoint` (`GameplayStatics.BreakHitResult` _outhit)) (`.ImpactNormal` (`GameplayStatics.BreakHitResult` _outhit)))
                (`self.K2_DestroyActor`))))))
      (:`Is Not Valid`
        (`KismetSystemLibrary.Delay` 10.0)
        (`self.K2_DestroyActor`)))))

(fn `UserConstructionScript`)