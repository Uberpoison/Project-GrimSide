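; Crossbow-wielding enemy character that spawns a crossbow into its hand socket and fires bolts through a Shoot event.
; Damage triggers blood effects, the health bar and a hit montage, and flags the player as seen on the blackboard.
; Death stops AI logic, disables collision and plays death montages.
; Tick hides the health bar, restarts AI when revived and clears sight when the player dies; Respawn resets blackboard state.
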(event `self.ReceiveTick`
  (params (DeltaSeconds :type "Float (single-precision)"))
  (bind _braincomponent (`AIController.BrainComponent` (`AIBlueprintHelperLibrary.GetAIController` self)))
  (bind _braincomponent_2 (`AIController.BrainComponent` (`AIBlueprintHelperLibrary.GetAIController` self)))
  (`parent.ReceiveTick` DeltaSeconds)
  (`|ExecutionSequence`
    (:`then_0`
      ;[1 1 1] disable health bar after a few seconds
      (if (and (`SceneComponent.IsVisible` (`self.HealthBar`)) (not (`self.IsTargeted`)))
        (`KismetSystemLibrary.Delay` (`self.HealthDisplayDuration`))
        (`self.ShowHealthBar` false)))
    (:`then_1`
      ;[1 1 1] If enemy isn't dead anymore restart AI and Enable Collision
      (if (`/Game/Blueprints/BPC_Health.IsDead` (`self.BPC_Health`))
        ;[1 1 1] If Enemy is dead check if BT is still running and play death anim
        (if (`BrainComponent.IsRunning` _braincomponent)
          (`BrainComponent.StopLogic` _braincomponent ""))
        (if (`self.ShouldPlayDeathAnim`)
          (`AnimInstance.Montage_Play` (`SkeletalMeshComponent.GetAnimInstance` (`self.Mesh`)) "/Game/Enemies/CrossbowEnemy/Animation/MON_CrossbowenemyStayDead.MON_CrossbowenemyStayDead" 1.0 "MontageLength" 0.0 true)
          (set `self.ShouldPlayDeathAnim` true))
        (else
          (set `self.ShouldPlayDeathAnim` false)
          (if (not (`BrainComponent.IsRunning` _braincomponent_2))
            (`BrainComponent.RestartLogic` _braincomponent_2)
            (`PrimitiveComponent.SetCollisionEnabled` (`self.CapsuleComponent`) "QueryAndPhysics")))))
    (:`then_2`
      (if (`/Game/Blueprints/BPC_Health.IsDead` (`/Game/Blueprints/BP_BaseCharacter.BPC_Health` (`self.Player`)))
        (`BlackboardComponent.SetValueAsBool` (`AIBlueprintHelperLibrary.GetBlackboard` null) (`self.CanSeePlayer`) false)))))

(event `self.ReceiveBeginPlay`
  (`parent.ReceiveBeginPlay`)
  (bind _returnvalue (`|SpawnActorFromClass` "/Game/Blueprints/AI/CrossbowEnemy/BP_Crossbow.BP_Crossbow_C" (`SceneComponent.K2_GetComponentToWorld` (`self.Mesh`)) "Undefined" "OverrideRootScale" null null))
  (bind _output_get (set `self.CurrentWeapon` _returnvalue))
  (`self.K2_AttachToComponent` _output_get (`self.Mesh`) "WeaponSocket" "SnapToTarget" "SnapToTarget" "KeepRelative" true)
  (bind _asbp_player_character (cast `/Game/Blueprints/BP_PlayerCharacter` (`GameplayStatics.GetPlayerPawn` 0)))
  (set `self.Player` _asbp_player_character))

(event `self.BPC_Health.OnTakingDamage`
  (params (DamageAmount :type "Float (single-precision)") (ImpactPoint :type "Vector Structure") (ImpactNormal :type "Vector Structure"))
  (bind _returnvalue (`NiagaraFunctionLibrary.SpawnSystemAtLocation` "/Game/FX/Particles/BloodSplash.BloodSplash" ImpactPoint (`KismetMathLibrary.MakeRotFromZ` ImpactNormal)))
  (`GameplayStatics.SpawnSoundAttached` "/Game/Audio/Gush.Gush" _returnvalue "None" (0.0 0.0 0.0) (struct) "KeepRelativeOffset" false 1.0 1.0 0.0 null null)
  ;[1 1 1] Show health bar and play hit animation
  (`self.ShowHealthBar` true)
  (if (not (`/Game/Blueprints/BPC_Health.IsDead` (`self.BPC_Health`)))
    (`AnimInstance.Montage_Play` (`SkeletalMeshComponent.GetAnimInstance` (`self.Mesh`)) "/Game/Enemies/CrossbowEnemy/Animation/MON_Hit.MON_Hit" 1.0 "MontageLength" 0.0 true)
    (`BlackboardComponent.SetValueAsBool` (`AIBlueprintHelperLibrary.GetBlackboard` null) (`self.CanSeePlayer`) true)))

(event `self.BPC_Health.OnDeath`
  (bind _returnvalue (`AIBlueprintHelperLibrary.GetAIController` self))
  (set `self.CanBeTargeted` false)
  (`AIController.K2_SetFocus` _returnvalue null)
  (`BrainComponent.StopLogic` (`AIController.BrainComponent` _returnvalue) "")
  (`PrimitiveComponent.SetCollisionEnabled` (`self.CapsuleComponent`) "NoCollision")
  (bind _returnvalue_2 (`AnimInstance.Montage_Play` (`SkeletalMeshComponent.GetAnimInstance` (`self.Mesh`)) "/Game/Enemies/CrossbowEnemy/Animation/MON_Death.MON_Death" 1.0 "MontageLength" 0.0 true))
  (`KismetSystemLibrary.Delay` (- _returnvalue_2 0.2))
  (set `self.ShouldPlayDeathAnim` true))

(event `self.LockOn`
  (`parent.LockOn`)
  (`self.ShowHealthBar` true))

(event `/Game/Blueprints/AI/BPI_Combat.Shoot`
  (`AnimInstance.Montage_Play` (`SkeletalMeshComponent.GetAnimInstance` (`self.Mesh`)) "/Game/Enemies/CrossbowEnemy/Animation/MON_Shoot.MON_Shoot" 1.0 "MontageLength" 0.0 true)
  (bind _asbp_crossbow (cast `/Game/Blueprints/AI/CrossbowEnemy/BP_Crossbow` (`self.CurrentWeapon`)))
  (`/Game/Blueprints/AI/CrossbowEnemy/BP_Crossbow.FireBolt` _asbp_crossbow))

(fn `Respawn`
  (bind _returnvalue (`AIBlueprintHelperLibrary.GetBlackboard` null))
  (`parent.Respawn`)
  (`BlackboardComponent.SetValueAsBool` _returnvalue (`self.CanSeePlayer`) false)
  (`BlackboardComponent.SetValueAsEnum` _returnvalue (`self.State`) (enumliteral `/Game/Blueprints/AI/ZombieEnemy/ENUM_AIState` "NewEnumerator0"))
  (`BrainComponent.RestartLogic` (`AIController.BrainComponent` (`AIBlueprintHelperLibrary.GetAIController` self))))

(fn `UserConstructionScript`
  (`parent.UserConstructionScript`))