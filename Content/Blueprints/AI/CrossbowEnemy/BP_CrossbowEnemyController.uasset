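; AI controller for the crossbow enemy that runs BT_CrossbowEnemy and feeds its blackboard with patrol and player-sighting data.
; BeginPlay copies the pawn's patrol path settings to the blackboard.
; Perception sets player visibility and AI state, with a timer delaying loss of sight so the chase persists briefly.
; Time-rewind overrides make the enemy unhittable during rewind and restore hittability and death animation on forward.
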(event `self.ReceiveBeginPlay`
  (bind _returnvalue (`AIBlueprintHelperLibrary.GetBlackboard` null))
  (`parent.ReceiveBeginPlay`)
  (bind _asbp_base_character (cast `/Game/Blueprints/BP_BaseCharacter` (`self.K2_GetPawn`)))
  (bind _output_get (set `self.MyPawn` _asbp_base_character))
  ;[1 1 1] Check if enemy has a patrolpath
  (`/Engine/EditorBlueprintResources/StandardMacros.IsValid` (`/Game/Blueprints/BP_BaseCharacter.PatrolPath` _output_get)
    (:`Is Valid`
      (`BlackboardComponent.SetValueAsBool` _returnvalue "HasPatrolPath" true)
      (`BlackboardComponent.SetValueAsBool` _returnvalue "PathLooping" (`/Game/Blueprints/AI/PatrolPath.IsLooping` (`/Game/Blueprints/BP_BaseCharacter.PatrolPath` (`self.MyPawn`))))
      (`BlackboardComponent.SetValueAsInt` _returnvalue "Direction" 1))
    (:`Is Not Valid`
      (`BlackboardComponent.SetValueAsBool` (`AIBlueprintHelperLibrary.GetBlackboard` null) "HasPatrolPath" false))))

(event `self.ReceiveTick`
  (params (DeltaSeconds :type "Float (single-precision)"))
  (`parent.ReceiveTick` DeltaSeconds)
  (if (`self.IsRewinding`)
    _))

(event `self.ReceivePossess`
  (params (PossessedPawn :type "Pawn Object Reference"))
  (`self.RunBehaviorTree` "/Game/Blueprints/AI/CrossbowEnemy/BT_CrossbowEnemy.BT_CrossbowEnemy"))

(event `self.AIPerception.OnTargetPerceptionUpdated`
  (params (Actor :type "Actor Object Reference") (Stimulus :type "AIStimulus Structure"))
  (bind _returnvalue (`AIBlueprintHelperLibrary.GetBlackboard` null))
  ;[1 1 1] Check if enemy can see player. if enemy loses sight of player set timer so that enemy doesnt give up chase immediately
  (cast `/Game/Blueprints/BP_PlayerCharacter` Actor)
  (if (`.bSuccessfullySensed` (break `AIStimulus` Stimulus))
    (`KismetSystemLibrary.K2_ClearAndInvalidateTimerHandle` (`self.EnemyTimer`))
    (`BlackboardComponent.SetValueAsBool` _returnvalue (`self.CanSeePlayer`) true)
    (`BlackboardComponent.SetValueAsEnum` _returnvalue (`self.State`) (enumliteral `/Game/Blueprints/AI/ZombieEnemy/ENUM_AIState` "NewEnumerator1"))
    (else
      (bind _returnvalue_2 (`KismetSystemLibrary.K2_SetTimerDelegate` (delegate `StartEnemyTimer`) (`self.Line of Sight Timer`)))
      (set `self.EnemyTimer` _returnvalue_2))))

(event `StartEnemyTimer`
  (bind _returnvalue (`AIBlueprintHelperLibrary.GetBlackboard` null))
  ;[1 1 1] Check if enemy can see player. if enemy loses sight of player set timer so that enemy doesnt give up chase immediately
  (`BlackboardComponent.SetValueAsBool` _returnvalue (`self.CanSeePlayer`) false)
  (`BlackboardComponent.SetValueAsEnum` _returnvalue (`self.State`) (enumliteral `/Game/Blueprints/AI/ZombieEnemy/ENUM_AIState` "NewEnumerator0")))

(event `/Game/Blueprints/BPI_TimeControl.Forward`
  (`parent.Forward`)
  (bind _asbp_crossbow_enemy (cast `/Game/Blueprints/AI/CrossbowEnemy/BP_CrossbowEnemy` (`self.MyPawn`)))
  (set `/Game/Blueprints/AI/CrossbowEnemy/BP_CrossbowEnemy.ShouldPlayDeathAnim` true _asbp_crossbow_enemy)
  (set `/Game/Blueprints/BP_BaseCharacter.CanBeHit` true _asbp_crossbow_enemy))

(event `/Game/Blueprints/BPI_TimeControl.Rewind`
  (`parent.Rewind`)
  (bind _asbp_crossbow_enemy (cast `/Game/Blueprints/AI/CrossbowEnemy/BP_CrossbowEnemy` (`self.MyPawn`)))
  (set `/Game/Blueprints/BP_BaseCharacter.CanBeHit` false _asbp_crossbow_enemy))

(fn `UserConstructionScript`
  (`parent.UserConstructionScript`))