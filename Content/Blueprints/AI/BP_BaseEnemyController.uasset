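; Base enemy controller that lets its pawn rewind through time.
; Each Tick it records transform, health and velocity, plus montages at the frame they stop, indexed alongside the transforms.
; While rewinding it pops those arrays newest-first to restore state and feed movement input, playing montages backwards from their end.
; Rewind stops the AI brain logic, Forward restarts it, and ClearRewindArrays wipes the history.
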(event `self.ReceiveTick`
  (params (DeltaSeconds :type "Float (single-precision)"))
  (bind _actortransforms (`self.ActorTransforms`))
  (bind _animmontages (`self.AnimMontages`))
  (bind _animmontages_2 (`self.AnimMontages`))
  (bind _tempmontage (`self.TempMontage`))
  (bind _animlength (`self.animLength`))
  (bind _animlength_2 (`self.animLength`))
  (bind _actorvelocities (`self.ActorVelocities`))
  (bind _actorvelocities_2 (`self.ActorVelocities`))
  (bind _actorvelocities_3 (`self.ActorVelocities`))
  (bind _healthstates (`self.HealthStates`))
  (bind _actortransforms_2 (`self.ActorTransforms`))
  (bind _healthstates_2 (`self.HealthStates`))
  (bind _healthstates_3 (`self.HealthStates`))
  (bind _actortransforms_3 (`self.ActorTransforms`))
  (bind _returnvalue (`KismetArrayLibrary.Array_LastIndex` _actortransforms_2))
  (bind _returnvalue_2 (`KismetArrayLibrary.Array_LastIndex` _actorvelocities_3))
  (bind _returnvalue_3 (`KismetArrayLibrary.Array_LastIndex` _healthstates_3))
  (bind _returnvalue_4 (`KismetArrayLibrary.Array_LastIndex` _animmontages))
  (bind _returnvalue_5 (`KismetArrayLibrary.Array_LastIndex` _animmontages_2))
  (bind _returnvalue_6 (`KismetArrayLibrary.Array_LastIndex` _animlength_2))
  (bind _returnvalue_7 (`KismetArrayLibrary.Array_LastIndex` (`self.ActorTransforms`)))
  (bind _returnvalue_8 (`SkeletalMeshComponent.GetAnimInstance` (`Character.Mesh` (`self.MyPawn`))))
  (bind _returnvalue_9 (`AnimInstance.GetCurrentActiveMontage` _returnvalue_8))
  ;[1 1 1] Rewind Time
  (`|ExecutionSequence`
    (:`then_0`
      ;;[1 1 1] If player isnt rewinding keep track of this actors position an animations
      (if (`self.IsRewinding`)
        (if (> (`KismetArrayLibrary.Array_LastIndex` (`self.ActorTransforms`)) 0)
          (`self.K2_SetActorTransform` (`self.MyPawn`) (`|GetArrayItem` _actortransforms_3 (`KismetArrayLibrary.Array_LastIndex` _actortransforms_3)) false false)
          (set `/Game/Blueprints/BPC_Health.CurrentHealth` (`|GetArrayItem` _healthstates (`KismetArrayLibrary.Array_LastIndex` _healthstates)) (`/Game/Blueprints/BP_BaseCharacter.BPC_Health` (`self.MyPawn`)))
          (`Pawn.AddMovementInput` (`self.MyPawn`) (`|GetArrayItem` _actorvelocities (`KismetArrayLibrary.Array_LastIndex` _actorvelocities)) 1.0 false)
          (if (== (`KismetArrayLibrary.Array_LastIndex` (`self.ActorTransforms`)) _returnvalue_5)
            (`AnimInstance.Montage_Play` (`SkeletalMeshComponent.GetAnimInstance` (`Character.Mesh` (`self.MyPawn`))) (`|GetArrayItem` _animmontages_2 _returnvalue_5) -1.0 "MontageLength" (`|GetArrayItem` _animlength (`KismetArrayLibrary.Array_LastIndex` _animlength)) true)
            (if (> _returnvalue_4 0)
              (`KismetArrayLibrary.Array_Remove` _animmontages _returnvalue_4)
              (if (> _returnvalue_6 0)
                (`KismetArrayLibrary.Array_Remove` _animlength_2 _returnvalue_6)
                (if (> _returnvalue 0) :!label _label
                  (`KismetArrayLibrary.Array_Remove` _actortransforms_2 _returnvalue)
                  (if (> _returnvalue_3 0)
                    (`KismetArrayLibrary.Array_Remove` _healthstates_3 _returnvalue_3)
                    (if (> _returnvalue_2 0)
                      (`KismetArrayLibrary.Array_Remove` _actorvelocities_3 _returnvalue_2))))))
            (else
              (goto _label)))
          (else
            (`self.K2_SetActorTransform` (`self.MyPawn`) (`|GetArrayItem` _actortransforms (`KismetArrayLibrary.Array_LastIndex` _actortransforms)) false false)
            (set `/Game/Blueprints/BPC_Health.CurrentHealth` (`|GetArrayItem` _healthstates_2 (`KismetArrayLibrary.Array_LastIndex` _healthstates_2)) (`/Game/Blueprints/BP_BaseCharacter.BPC_Health` (`self.MyPawn`)))
            (`Pawn.AddMovementInput` (`self.MyPawn`) (`|GetArrayItem` _actorvelocities_2 (`KismetArrayLibrary.Array_LastIndex` _actorvelocities_2)) 1.0 false)))
        (else
          (`KismetArrayLibrary.Array_Add` (`self.ActorTransforms`) (`self.GetTransform` (`self.MyPawn`)))
          (`KismetArrayLibrary.Array_Add` (`self.HealthStates`) (`/Game/Blueprints/BPC_Health.CurrentHealth` (`/Game/Blueprints/BP_BaseCharacter.BPC_Health` (`self.MyPawn`))))
          (`KismetArrayLibrary.Array_Add` (`self.ActorVelocities`) (`self.GetVelocity` (`self.MyPawn`)))
          (if (`AnimInstance.IsAnyMontagePlaying` (`SkeletalMeshComponent.GetAnimInstance` (`Character.Mesh` (`self.MyPawn`))))
            (if (`self.ShouldAddMontage`)
              (if (`AnimInstance.Montage_IsPlaying` _returnvalue_8 _returnvalue_9)
                (set `self.TempMontage` _returnvalue_9)
                (else
                  (`KismetArrayLibrary.Array_Set` (`self.AnimMontages`) _returnvalue_7 _tempmontage true)
                  (bind _returnvalue_10 (`AnimSequenceBase.GetPlayLength` _tempmontage))
                  (`KismetArrayLibrary.Array_Set` (`self.animLength`) _returnvalue_7 _returnvalue_10 true)
                  (set `self.ShouldAddMontage` false)
                  (set `self.TempMontage` null))))
            (else
              (set `self.ShouldAddMontage` true))))))))

(event `self.ReceiveBeginPlay`)

(event `/Game/Blueprints/BPI_TimeControl.Rewind`
  (bind _returnvalue (`AIBlueprintHelperLibrary.GetAIController` (`self.MyPawn`)))
  ;[1 1 1] Rewind
  (set `self.IsRewinding` true)
  (`/Engine/EditorBlueprintResources/StandardMacros.IsValid` _returnvalue
    (:`Is Valid`
      (`BrainComponent.StopLogic` (`AIController.BrainComponent` _returnvalue) ""))))

(event `/Game/Blueprints/BPI_TimeControl.Forward`
  (bind _returnvalue (`AIBlueprintHelperLibrary.GetAIController` (`self.MyPawn`)))
  (bind _braincomponent (`AIController.BrainComponent` _returnvalue))
  ;[1 1 1] Forward
  (set `self.IsRewinding` false)
  (`/Engine/EditorBlueprintResources/StandardMacros.IsValid` _returnvalue
    (:`Is Valid`
      (if (not (`BrainComponent.IsRunning` _braincomponent))
        (`BrainComponent.RestartLogic` _braincomponent)))))

(fn `ClearRewindArrays`
  (`KismetArrayLibrary.Array_Clear` (`self.ActorTransforms`))
  (`KismetArrayLibrary.Array_Clear` (`self.ActorVelocities`))
  (`KismetArrayLibrary.Array_Clear` (`self.AnimMontages`))
  (`KismetArrayLibrary.Array_Clear` (`self.animLength`))
  (`KismetArrayLibrary.Array_Clear` (`self.HealthStates`)))

(fn `UserConstructionScript`)