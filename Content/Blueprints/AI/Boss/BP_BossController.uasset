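; BP_BossController is the boss's AI controller, running the BT_Boss behavior tree on possession.
; AI perception sets CanSeePlayer and changes the blackboard State when the player is sensed; losing sight still leaves CanSeePlayer true.
; Inherited Forward and Rewind events toggle whether the boss can be hit, with Forward also enabling its death animation.
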(event `self.ReceiveBeginPlay`
  (`parent.ReceiveBeginPlay`)
  (bind _asbp_base_character (cast `/Game/Blueprints/BP_BaseCharacter` (`self.K2_GetPawn`)))
  (set `self.MyPawn` _asbp_base_character))

(event `self.ReceivePossess`
  (params (PossessedPawn :type "Pawn Object Reference"))
  (`self.RunBehaviorTree` "/Game/Blueprints/AI/Boss/BT_Boss.BT_Boss"))

(event `self.AIPerception.OnTargetPerceptionUpdated`
  (params (Actor :type "Actor Object Reference") (Stimulus :type "AIStimulus Structure"))
  (bind _returnvalue (`AIBlueprintHelperLibrary.GetBlackboard` null))
  (cast `/Game/Blueprints/BP_PlayerCharacter` Actor)
  (if (`.bSuccessfullySensed` (break `AIStimulus` Stimulus))
    (`BlackboardComponent.SetValueAsBool` _returnvalue (`self.CanSeePlayer`) true)
    (`BlackboardComponent.SetValueAsEnum` _returnvalue (`self.State`) (enumliteral `/Game/Blueprints/AI/ZombieEnemy/ENUM_AIState` "NewEnumerator2"))
    (else
      (`BlackboardComponent.SetValueAsBool` _returnvalue (`self.CanSeePlayer`) true))))

(event `self.Forward`
  (`parent.Forward`)
  (bind _asbp_boss (cast `/Game/Blueprints/AI/Boss/BP_Boss` (`self.MyPawn`)))
  (set `/Game/Blueprints/AI/Boss/BP_Boss.ShouldPlayDeathAnim` true _asbp_boss)
  (set `/Game/Blueprints/BP_BaseCharacter.CanBeHit` true _asbp_boss))

(event `self.Rewind`
  (`parent.Rewind`)
  (bind _asbp_boss (cast `/Game/Blueprints/AI/Boss/BP_Boss` (`self.MyPawn`)))
  (set `/Game/Blueprints/BP_BaseCharacter.CanBeHit` false _asbp_boss))

(fn `UserConstructionScript`
  (`parent.UserConstructionScript`))