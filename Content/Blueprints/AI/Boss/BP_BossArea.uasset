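; Boss arena trigger that shows a boss info widget and plays the boss theme while the player is inside.
; BeginPlay caches the player and creates the widget, and collision overlaps set the in-area and should-add-effects flags.
; Tick uses those flags to add effects once for a living boss and remove them when it dies.
; Leaving the area also removes the widget and stops the music after a short delay.
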(event `self.ReceiveBeginPlay`
  (bind _returnvalue (`GameplayStatics.GetPlayerPawn` 0))
  (`/Engine/EditorBlueprintResources/StandardMacros.IsValid` _returnvalue
    (:`Is Valid`
      (bind _asbp_player_character (cast `/Game/Blueprints/BP_PlayerCharacter` _returnvalue))
      (set `self.Player` _asbp_player_character)
      (bind _returnvalue_2 (`|CreateWidget` "/Game/Blueprints/BP_BossInfo.BP_BossInfo_C"))
      (set `self.BossInfo` _returnvalue_2)
      (`AudioComponent.Stop` (`self.BossTheme`)))))

(event `self.ReceiveTick`
  (params (DeltaSeconds :type "Float (single-precision)"))
  (if (`self.PlayerIsInBossArea`)
    (if (`self.ShouldAddEffects`)
      (if (`/Game/Blueprints/BPC_Health.IsDead` (`/Game/Blueprints/BP_BaseCharacter.BPC_Health` (`self.Boss`)))
        (`self.RemoveEffects`)
        (else
          (`self.AddEffects`)))
      (elif (`/Game/Blueprints/BPC_Health.IsDead` (`/Game/Blueprints/BP_BaseCharacter.BPC_Health` (`self.Boss`)))
        (`self.RemoveEffects`)))))

(event `self.CollisionComponent.OnComponentBeginOverlap`
  (params (OverlappedComponent :type "PrimitiveComponent Object Reference") (OtherActor :type "Actor Object Reference") (OtherComp :type "PrimitiveComponent Object Reference") (OtherBodyIndex :type Integer) (bFromSweep :type Boolean) (SweepResult :type "HitResult Structure (by ref)"))
  (bind _asbp_player_character (cast `/Game/Blueprints/BP_PlayerCharacter` OtherActor))
  (if (== _asbp_player_character (`self.Player`))
    (set `self.PlayerIsInBossArea` true)
    (set `self.ShouldAddEffects` true)))

(event `self.CollisionComponent.OnComponentEndOverlap`
  (params (OverlappedComponent :type "PrimitiveComponent Object Reference") (OtherActor :type "Actor Object Reference") (OtherComp :type "PrimitiveComponent Object Reference") (OtherBodyIndex :type Integer))
  (bind _asbp_player_character (cast `/Game/Blueprints/BP_PlayerCharacter` OtherActor))
  (if (== _asbp_player_character (`self.Player`))
    (set `self.PlayerIsInBossArea` false)
    (set `self.ShouldAddEffects` false)
    (`self.RemoveEffects`)))

(fn `AddEffects`
  (bind _bossinfo (`self.BossInfo`))
  (`|ExecutionSequence`
    (:`then_0`
      (set `/Game/Blueprints/BP_BossInfo.Boss` (`self.Boss`) _bossinfo)
      (`UserWidget.AddToViewport` _bossinfo 0))
    (:`then_1`
      (`AudioComponent.Play` (`self.BossTheme`) 0.0)
      (set `self.ShouldAddEffects` false))))

(fn `RemoveEffects`
  (bind _bosstheme (`self.BossTheme`))
  (`|ExecutionSequence`
    (:`then_0`
      (`Widget.RemoveFromParent` (`self.BossInfo`)))
    (:`then_1`
      (if (`AudioComponent.IsPlaying` _bosstheme)
        (`AudioComponent.StopDelayed` _bosstheme 2.0)
        (set `self.ShouldAddEffects` true)))))

(fn `UserConstructionScript`)