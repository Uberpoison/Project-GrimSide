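; Troll melee enemy built on a parent enemy class, spawning with a hammer in hand and driven by a behavior tree.
; MeleeAttack plays one of six random attack montages, while taking damage spawns blood and sound, shows the health bar and sets CanSeePlayer on the blackboard.
; Death stops AI logic and capsule collision, then Tick holds the dead pose, restores both upon revival and clears player sight when the player dies.
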(event `self.ReceiveTick`
  (params (DeltaSeconds :type "Float (single-precision)"))
  (bind _braincomponent (`AIController.BrainComponent` (`AIBlueprintHelperLibrary.GetAIController` self)))
  (bind _braincomponent_2 (`AIController.BrainComponent` (`AIBlueprintHelperLibrary.GetAIController` self)))
  (`parent.ReceiveTick` DeltaSeconds)
  (`|ExecutionSequence`
    (:`then_0`
      ;[1 1 1] disable health bar after a few seconds
      (if (and (`SceneComponent.IsVisible` (`self.HealthBar`)) (not (`self.IsTargeted`)))
        (`KismetSystemLibrary.Delay` (`self.HealthDisplayDuration`))
        (`self.ShowHealthBar` false)))
    (:`then_1`
      ;[1 1 1] If enemy isn't dead anymore restart AI and Enable Collision
      (if (`/Game/Blueprints/BPC_Health.IsDead` (`self.BPC_Health`))
        ;[1 1 1] If Enemy is dead check if BT is still running and play death anim
        (if (`BrainComponent.IsRunning` _braincomponent)
          (`BrainComponent.StopLogic` _braincomponent ""))
        (if (`self.ShouldPlayDeathAnim`)
          (`AnimInstance.Montage_Play` (`SkeletalMeshComponent.GetAnimInstance` (`self.Mesh`)) "/Game/Enemies/Enemy_Troll/Enemy_Troll_Poison_Animation/MON_TrollStayDead.MON_TrollStayDead" 1.0 "MontageLength" 0.0 true)
          (set `self.ShouldPlayDeathAnim` true))
        (else
          (set `self.ShouldPlayDeathAnim` false)
          (if (not (`BrainComponent.IsRunning` _braincomponent_2))
            (`BrainComponent.RestartLogic` _braincomponent_2)
            (`PrimitiveComponent.SetCollisionEnabled` (`self.CapsuleComponent`) "QueryAndPhysics")))))
    (:`then_2`
      (if (`/Game/Blueprints/BPC_Health.IsDead` (`/Game/Blueprints/BP_BaseCharacter.BPC_Health` (`self.Player`)))
        (`BlackboardComponent.SetValueAsBool` (`AIBlueprintHelperLibrary.GetBlackboard` null) (`self.CanSeePlayer`) false)))))

(event `self.ReceiveBeginPlay`
  (`parent.ReceiveBeginPlay`)
  (bind _returnvalue (`|SpawnActorFromClass` "/Game/Blueprints/AI/TrollEnemy/BP_TrollHammer.BP_TrollHammer_C" (`SceneComponent.K2_GetComponentToWorld` (`self.Mesh`)) "Undefined" "OverrideRootScale" null null))
  (bind _output_get (set `self.CurrentWeapon` _returnvalue))
  (`self.K2_AttachToComponent` _output_get (`self.Mesh`) "b_MF_Weapon_R_Socket" "SnapToTarget" "SnapToTarget" "KeepRelative" true)
  (bind _asbp_player_character (cast `/Game/Blueprints/BP_PlayerCharacter` (`GameplayStatics.GetPlayerPawn` 0)))
  (set `self.Player` _asbp_player_character))

(event `/Game/Blueprints/AI/BPI_Combat.MeleeAttack`
  (switch `int` (`KismetMathLibrary.RandomInteger` 6)
    (:`0`
      (`AnimInstance.Montage_Play` (`SkeletalMeshComponent.GetAnimInstance` (`self.Mesh`)) "/Game/Enemies/Enemy_Troll/Enemy_Troll_Poison_Animation/MON_TrollAttack01.MON_TrollAttack01" (`self.AttackSpeedMultiplier`) "MontageLength" 0.0 true))
    (:`1`
      (`AnimInstance.Montage_Play` (`SkeletalMeshComponent.GetAnimInstance` (`self.Mesh`)) "/Game/Enemies/Enemy_Troll/Enemy_Troll_Poison_Animation/MON_TrollAttack02.MON_TrollAttack02" (`self.AttackSpeedMultiplier`) "MontageLength" 0.0 true))
    (:`2`
      (`AnimInstance.Montage_Play` (`SkeletalMeshComponent.GetAnimInstance` (`self.Mesh`)) "/Game/Enemies/Enemy_Troll/Enemy_Troll_Poison_Animation/MON_TrollCharge.MON_TrollCharge" (`self.AttackSpeedMultiplier`) "MontageLength" 0.0 true))
    (:`3`
      (`AnimInstance.Montage_Play` (`SkeletalMeshComponent.GetAnimInstance` (`self.Mesh`)) "/Game/Enemies/Enemy_Troll/Enemy_Troll_Poison_Animation/MON_TrollCombo01.MON_TrollCombo01" (`self.AttackSpeedMultiplier`) "MontageLength" 0.0 true))
    (:`4`
      (`AnimInstance.Montage_Play` (`SkeletalMeshComponent.GetAnimInstance` (`self.Mesh`)) "/Game/Enemies/Enemy_Troll/Enemy_Troll_Poison_Animation/MON_TrollCombo02.MON_TrollCombo02" (`self.AttackSpeedMultiplier`) "MontageLength" 0.0 true))
    (:`5`
      (`AnimInstance.Montage_Play` (`SkeletalMeshComponent.GetAnimInstance` (`self.Mesh`)) "/Game/Enemies/Enemy_Troll/Enemy_Troll_Poison_Animation/MON_TrollOverheadAttack.MON_TrollOverheadAttack" (`self.AttackSpeedMultiplier`) "MontageLength" 0.0 true))))

(event `self.BPC_Health.OnTakingDamage`
  (params (DamageAmount :type "Float (single-precision)") (ImpactPoint :type "Vector Structure") (ImpactNormal :type "Vector Structure"))
  (bind _returnvalue (`NiagaraFunctionLibrary.SpawnSystemAtLocation` "/Game/FX/Particles/BloodSplash.BloodSplash" ImpactPoint (`KismetMathLibrary.MakeRotFromZ` ImpactNormal)))
  (`GameplayStatics.SpawnSoundAttached` "/Game/Audio/Gush.Gush" _returnvalue "None" (0.0 0.0 0.0) (struct) "KeepRelativeOffset" false 1.0 1.0 0.0 null null)
  ;[1 1 1] Show health bar
  (`self.ShowHealthBar` true)
  (if (not (`/Game/Blueprints/BPC_Health.IsDead` (`self.BPC_Health`)))
    (`BlackboardComponent.SetValueAsBool` (`AIBlueprintHelperLibrary.GetBlackboard` null) (`self.CanSeePlayer`) true)))

(event `self.BPC_Health.OnDeath`
  (set `self.CanBeTargeted` false)
  ;[1 1 1] stop logic and disable collision on death
  (`BrainComponent.StopLogic` (`AIController.BrainComponent` (`AIBlueprintHelperLibrary.GetAIController` self)) "")
  (`PrimitiveComponent.SetCollisionEnabled` (`self.CapsuleComponent`) "NoCollision")
  (bind _returnvalue (`AnimInstance.Montage_Play` (`SkeletalMeshComponent.GetAnimInstance` (`self.Mesh`)) "/Game/Enemies/Enemy_Troll/Enemy_Troll_Poison_Animation/MON_TrollDeath.MON_TrollDeath" 1.0 "MontageLength" 0.0 true))
  (`KismetSystemLibrary.Delay` (- _returnvalue 0.2))
  (set `self.ShouldPlayDeathAnim` true))

(event `self.LockOn`
  (`parent.LockOn`)
  (`self.ShowHealthBar` true))

(fn `Respawn`
  (bind _returnvalue (`AIBlueprintHelperLibrary.GetBlackboard` null))
  (`parent.Respawn`)
  (`BlackboardComponent.SetValueAsBool` _returnvalue (`self.CanSeePlayer`) false)
  (`BlackboardComponent.SetValueAsEnum` _returnvalue (`self.State`) (enumliteral `/Game/Blueprints/AI/ZombieEnemy/ENUM_AIState` "NewEnumerator0"))
  (`BrainComponent.RestartLogic` (`AIController.BrainComponent` (`AIBlueprintHelperLibrary.GetAIController` self))))

(fn `UserConstructionScript`
  (`parent.UserConstructionScript`))