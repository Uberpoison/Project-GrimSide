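; BP_CheckPoint is a rest-point actor that, on interact, sets the player's spawn point, resets health, stamina and time mana, and respawns enemies.
; Tick compares player distance to UsableDistance, rather than using trigger overlaps, to toggle input and the interact prompt widget.
; Interacting respawns every other BP_BaseCharacter and clears enemy controllers' rewind data.
; It then plays a smoke effect while input is locked for a short delay.
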(event `self.ReceiveBeginPlay`
  (bind _returnvalue (`GameplayStatics.GetPlayerPawn` 0))
  ;[1 1 1] BeginPlay
  (bind _asbp_player_character (cast `/Game/Blueprints/BP_PlayerCharacter` _returnvalue))
  (set `self.Player` _asbp_player_character)
  (bind _asbp_player_controller (cast `/Game/Blueprints/BP_PlayerController` (`Pawn.GetController` _returnvalue)))
  (set `self.PlayerController` _asbp_player_controller)
  (bind _returnvalue_2 (`|CreateWidget` "/Game/Blueprints/BP_InteractPrompt.BP_InteractPrompt_C"))
  (set `self.InteractPrompt` _returnvalue_2))

(event `self.ReceiveTick`
  (params (DeltaSeconds :type "Float (single-precision)"))
  ;[1 1 1] Event Tick
  (if (<= (`KismetMathLibrary.Vector_Distance` (`self.K2_GetActorLocation` self) (`self.K2_GetActorLocation` (`self.Player`))) (`self.UsableDistance`))
    (set `self.PlayerIsInTrigger` true)
    (`self.EnableInput` (`self.PlayerController`))
    (if (`self.ShouldAddToViewPoer`)
      (`UserWidget.AddToViewport` (`self.InteractPrompt`) 0)
      (set `self.ShouldAddToViewPoer` false))
    (else
      (set `self.PlayerIsInTrigger` false)
      (`self.DisableInput` (`self.PlayerController`))
      (if (not (`self.ShouldAddToViewPoer`))
        (`Widget.RemoveFromParent` (`self.InteractPrompt`))
        (set `self.ShouldAddToViewPoer` true)))))

(event `self.Trigger.OnComponentBeginOverlap`
  (params (OverlappedComponent :type "PrimitiveComponent Object Reference") (OtherActor :type "Actor Object Reference") (OtherComp :type "PrimitiveComponent Object Reference") (OtherBodyIndex :type Integer) (bFromSweep :type Boolean) (SweepResult :type "HitResult Structure (by ref)")))

(event `self.Trigger.OnComponentEndOverlap`
  (params (OverlappedComponent :type "PrimitiveComponent Object Reference") (OtherActor :type "Actor Object Reference") (OtherComp :type "PrimitiveComponent Object Reference") (OtherBodyIndex :type Integer)))

(event `InputAction|Interact`
  (params (Key :type "Key Structure"))
  (bind _playercontroller (`self.PlayerController`))
  (bind _p_smoking1 (`self.P_Smoking1`))
  (bind _playercontroller_2 (`self.PlayerController`))
  ;[1 1 1] When the player presses the interact button reset player stats and respawn enemies
  (:`Pressed`
    (if (`self.PlayerIsInTrigger`)
      (`self.SetNewSpawnPoint`)
      (`self.ResetPlayerStats`)
      (`self.RespawnEnemies`)
      (`ActorComponent.Activate` _p_smoking1 false)
      (`self.DisableInput` _playercontroller)
      (`self.DisableInput` _playercontroller _playercontroller)
      (`Widget.RemoveFromParent` (`self.InteractPrompt`))
      (`KismetSystemLibrary.Delay` 2.0)
      (`ActorComponent.Deactivate` _p_smoking1)
      (`self.EnableInput` _playercontroller_2)
      (`self.EnableInput` _playercontroller_2 _playercontroller_2))))

(event `SetNewSpawnPoint`
  ;[1 1 1] SetNewSpawnPoint
  (`/Game/Blueprints/BP_BaseCharacter.SetSpawnPoint` (`self.Player`) (`KismetMathLibrary.MakeTransform` (+ (.location (`SceneComponent.K2_GetComponentToWorld` (`self.Mesh`))) (`self.NewPlayerSpawnPoint`)) (.rotation (`SceneComponent.K2_GetComponentToWorld` (`self.Mesh`))))))

(event `RespawnEnemies`
  ;[1 1 1] RespawnEnemies
  (bind _outactors (`GameplayStatics.GetAllActorsOfClass` "/Game/Blueprints/BP_BaseCharacter.BP_BaseCharacter_C"))
  (for _array_element _outactors
    (if (not (== _array_element (`self.Player`)))
      (`/Game/Blueprints/BP_BaseCharacter.Respawn` _array_element)))
  ;;[1 1 1] Clear Rewind Data of the Enemies
  (bind _outactors_2 (`GameplayStatics.GetAllActorsOfClass` "/Game/Blueprints/AI/BP_BaseEnemyController.BP_BaseEnemyController_C"))
  (for _array_element_2 _outactors_2
    (`/Game/Blueprints/AI/BP_BaseEnemyController.ClearRewindArrays` _array_element_2)))

(event `ResetPlayerStats`
  (bind _player (`self.Player`))
  ;[1 1 1] ResetPlayerStats
  (`/Game/Blueprints/BPC_Health.ResetHealth` (`/Game/Blueprints/BP_BaseCharacter.BPC_Health` _player))
  (`/Game/Blueprints/BP_PlayerCharacter.ResetStamina` _player)
  (`/Game/Blueprints/BP_PlayerCharacter.ResetTimeMana` _player))

(fn `UserConstructionScript`)